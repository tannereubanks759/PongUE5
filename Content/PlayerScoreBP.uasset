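; PlayerScoreBP keeps score for a two-player Pong game and announces the winner.
; Player1Scored and Player2Scored each increment their score and update that player's text display.
; When a score passes four, that player's win indicator becomes visible; otherwise a new Pong_Ball spawns at a random height to continue play.
; The event graph is empty, so scoring runs only when these functions are called from outside.
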(fn `Player1Scored`
  (bind _output_get (set `self.Score1` (+ (`self.Score1`) 1)))
  (`TextRenderComponent.K2_SetText` (`self.ScoreText`) (`KismetTextLibrary.Conv_IntToText` _output_get))
  (if (> (`self.Score1`) 4)
    (`SceneComponent.SetVisibility` (`self.Player1Wins`) true false)
    (else
      (`AIBlueprintHelperLibrary.SpawnAIFromClass` "/Game/Pong_Ball.Pong_Ball_C" null (`KismetMathLibrary.MakeVector` 0.0 0.0 (`KismetMathLibrary.RandomFloatInRange` -900.0 900.0)) (struct) false null))))

(fn `Player2Scored`
  (bind _output_get (set `self.Score2` (+ (`self.Score2`) 1)))
  (`TextRenderComponent.K2_SetText` (`self.Score2Text`) (`KismetTextLibrary.Conv_IntToText` _output_get))
  (if (> (`self.Score2`) 4)
    (`SceneComponent.SetVisibility` (`self.Player2Wins`) true false)
    (else
      (`AIBlueprintHelperLibrary.SpawnAIFromClass` "/Game/Pong_Ball.Pong_Ball_C" null (`KismetMathLibrary.MakeVector` 0.0 0.0 (`KismetMathLibrary.RandomFloatInRange` -900.0 900.0)) (struct) false null))))

(fn `UserConstructionScript`)